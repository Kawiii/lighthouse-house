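; BP_Clock is an office prop clock that shows the current system time by rotating its Hour and Min components.
; UpdateTime converts Now() into relative pitch rotations, so each hand moves in whole-unit steps with no minute offset on the hour hand.
; The construction script sets the hands on construction, and BeginPlay refreshes them in a one-second Delay loop instead of using Tick.
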(event EventBeginPlay
  (CallFunction|UpdateTime :!label _label)
  (Utilities|FlowControl|Delay 1.0)
  (goto _label))

(fn ConstructionScript
  (CallFunction|UpdateTime))

(fn UpdateTime
  (bind _returnvalue (Math|DateTime|Now))
  (bind (_year _month _day _hour _minute) (Math|DateTime|BreakDateTime _returnvalue))
  (Transformation|SetRelativeRotation (Variables|Default|GetHour) (Math|Rotator|MakeRotator 0.0 (* _hour -3e+01) 0.0) false false)
  (Transformation|SetRelativeRotation (Variables|Default|GetMin) (Math|Rotator|MakeRotator 0.0 (* _minute -6.0) 0.0) false false))