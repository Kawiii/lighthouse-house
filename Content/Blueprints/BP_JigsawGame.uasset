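; BP_JigsawGame is a one-shot interactable that starts a jigsaw game and leaves a photo item behind.
; Its construction script sizes the Sphere component from a radius variable and clears the interaction state.
; Interact calls PlayJigsaw on the interactor, destroys the actor and immediately spawns BP_ItemPhoto at the player character's position and rotation, without waiting for a puzzle result.
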(fn ConstructionScript
  (Components|Sphere|SetSphereRadius (Variables|Default|GetSphere) (Variables|Default|GetRadius_0) true)
  (Variables|Default|SetInteractionState_0 false))

(fn Interact
  (params (Interactor :type BP%20Lighthouse%20Character%20Object%20Reference))
  (bind _returnvalue (Game|GetPlayerCharacter 0))
  (Default|PlayJigsaw Interactor)
  (Actor|DestroyActor)
  (Game|SpawnActorfromClass "/Game/Blueprints/ItemsInspect/BP_ItemPhoto.BP_ItemPhoto_C" (Math|Transform|MakeTransform (Transformation|GetActorLocation _returnvalue) (Transformation|GetActorRotation _returnvalue)) "Undefined" "MultiplyWithRoot" 0 0)
  (return true))