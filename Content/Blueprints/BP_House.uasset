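; BP_House is a house actor that hides its roof while the lighthouse character is inside its trigger sphere.
; Sphere begin overlap by a BP_LighthouseCharacter hides the SMRoof component, and end overlap shows it again.
; Both events set the roof to NoCollision, so its collision stays off after the character leaves.
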(event OnComponentBeginOverlap(Sphere)
  (params (OverlappedComponent :type Primitive%20Component%20Object%20Reference) (OtherActor :type Actor%20Object%20Reference) (OtherComp :type Primitive%20Component%20Object%20Reference) (OtherBodyIndex :type Integer) (bFromSweep :type Boolean) (SweepResult :type Hit%20Result%20Structure%20%28by%20ref%29))
  (bind _sm_roof (Variables|Default|GetSM_Roof))
  (bind _asbp_lighthouse_character (Utilities|Casting|CastToBP_LighthouseCharacter OtherActor))
  (if (Utilities|IsValid _asbp_lighthouse_character)
    (Rendering|SetVisibility _sm_roof false false)
    (Collision|SetCollisionEnabled _sm_roof "NoCollision")))

(event OnComponentEndOverlap(Sphere)
  (params (OverlappedComponent :type Primitive%20Component%20Object%20Reference) (OtherActor :type Actor%20Object%20Reference) (OtherComp :type Primitive%20Component%20Object%20Reference) (OtherBodyIndex :type Integer))
  (bind _sm_roof (Variables|Default|GetSM_Roof))
  (bind _asbp_lighthouse_character (Utilities|Casting|CastToBP_LighthouseCharacter OtherActor))
  (if (Utilities|IsValid _asbp_lighthouse_character)
    (Rendering|SetVisibility _sm_roof true false)
    (Collision|SetCollisionEnabled _sm_roof "NoCollision")))

(event EventBeginPlay)

(event EventTick
  (params (DeltaSeconds :type Float%20%28single-precision%29)))

(fn ConstructionScript)