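; BP_Inspectitem is an actor that presents an inspected item to the player.
; Its Inspect event stores the character, sets the passed mesh on its Item component, and adds a W_Inspect widget showing the item's name and description to the viewport.
; It then disables and re-enables input for player controller 0.
; Its Interact function only returns false, and the construction script is empty.
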(event Custom|Inspect_1
  (params (Character :type BP%20Lighthouse%20Character%20Object%20Reference) (Inspected%20Item :type Static%20Mesh%20Object%20Reference) (Item%20Name :type Text) (Item%20Description :type Text))
  (bind _returnvalue (Game|GetPlayerController 0))
  (Variables|Default|SetCharacter Character)
  (Components|StaticMesh|SetStaticMesh (Variables|Default|GetItem) Inspected%20Item)
  (bind _returnvalue_2 (UserInterface|CreateWidget "/Game/Blueprints/Inspect/W_Inspect.W_Inspect_C" 0 Item%20Name Item%20Description))
  (bind _output_get (Variables|Default|SetInspectWidgetReference _returnvalue_2))
  (UserInterface|Viewport|AddtoViewport _output_get 0)
  (Input|DisableInput _returnvalue)
  (Input|EnableInput _returnvalue))

(fn ConstructionScript)

(fn Interact
  (params (Interactor :type BP%20Lighthouse%20Character%20Object%20Reference))
  (return false))