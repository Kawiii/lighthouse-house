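; BP_TeleportControl is an interactable, named as a teleport control, that is gated behind the lighthouse's wire and generator tasks.
; Interact casts the interactor to BP_LighthouseCharacter and reads both completion flags from its HUD widget.
; With both tasks done it disables the Box collision; otherwise the HUD shows the generator refuel prompt, cable repair prompt or both, matching what remains.
; No teleport logic appears in this Blueprint.
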(event EventBeginPlay
  (|CallParentFunction)
  (if true
    _))

(event Collision|EventActorBeginOverlap
  (params (OtherActor :type Actor%20Object%20Reference)))

(event EventTick
  (params (DeltaSeconds :type Float%20%28single-precision%29)))

(fn ConstructionScript
  (|CallParentFunction))

(fn Interact
  (params (Interactor :type BP%20Lighthouse%20Character%20Object%20Reference))
  (bind _asbp_lighthouse_character (Utilities|Casting|CastToBP_LighthouseCharacter Interactor))
  (if (Variables|/Game/Blueprints/WBP_HUD.WBP_HUD_C|GetWIRETASK_DONE (Variables|/Game/Blueprints/BP_LighthouseCharacter.BP_LighthouseCharacter_C|GetHUD_Widget _asbp_lighthouse_character))
    (if (Variables|/Game/Blueprints/WBP_HUD.WBP_HUD_C|GetGENERATOR_COMPLETE (Variables|/Game/Blueprints/BP_LighthouseCharacter.BP_LighthouseCharacter_C|GetHUD_Widget _asbp_lighthouse_character))
      (Collision|SetCollisionEnabled (Variables|Default|GetBox) "NoCollision")
      (return false)
      (else
        (Default|ShowGeneratorRefuel (Variables|/Game/Blueprints/BP_LighthouseCharacter.BP_LighthouseCharacter_C|GetHUD_Widget _asbp_lighthouse_character))))
    (elif (Variables|/Game/Blueprints/WBP_HUD.WBP_HUD_C|GetGENERATOR_COMPLETE (Variables|/Game/Blueprints/BP_LighthouseCharacter.BP_LighthouseCharacter_C|GetHUD_Widget _asbp_lighthouse_character))
      (Default|ShowCablesRepair (Variables|/Game/Blueprints/BP_LighthouseCharacter.BP_LighthouseCharacter_C|GetHUD_Widget _asbp_lighthouse_character))
      (else
        (Default|ShowGeneratorRefuel (Variables|/Game/Blueprints/BP_LighthouseCharacter.BP_LighthouseCharacter_C|GetHUD_Widget _asbp_lighthouse_character))
        (Default|ShowCablesRepair (Variables|/Game/Blueprints/BP_LighthouseCharacter.BP_LighthouseCharacter_C|GetHUD_Widget _asbp_lighthouse_character))))))