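; BP_Generator is an interactable generator Blueprint that is gated on fuel.
; When it has no fuel, Interact checks the interactor's inventory for a required item index, noted as the canister, and prints a message and returns false if absent.
; BeginPlay caches the mesh's relative location and Tick checks a shaking flag, but the shake, refuelling and success paths are not implemented.
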(event EventBeginPlay
  (Variables|Default|SetOriginalLocation (Variables|/Script/Engine.SceneComponent|GetRelativeLocation (Variables|Default|GetGenerator))))

(event EventTick
  (params (DeltaSeconds :type Float%20%28single-precision%29))
  (if (Variables|Default|GetIsShaking)
    _))

(fn ConstructionScript
  (|CallParentFunction))

(fn Interact
  (params (Interactor :type BP%20Lighthouse%20Character%20Object%20Reference))
  (if (not (Variables|Default|GetHasFuel))
    ;[0.15 0.09518 0 0.5] Podminka pro vlastnictvi itemu urciteho Indexu = canister na indexu 3
    (bind _output_get (Variables|Default|SetCharacter Interactor))
    (if (not (Utilities|Array|ContainsItem (Variables|/Game/Blueprints/BP_LighthouseCharacter.BP_LighthouseCharacter_C|GetInventory _output_get) (Variables|Default|GetRequiredItemIndex)))
      (Development|PrintString "You don't have a fuel canister.")
      (return false))))