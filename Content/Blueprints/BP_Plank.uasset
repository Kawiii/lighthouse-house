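; BP_Plank is a plank pickup that a character can collect by interacting with it.
; Interact checks whether the interactor is already carrying a plank; if not, it sets the interactor's plank state, destroys itself and returns false.
; The event graph holds only disabled default events, so all of the actor's own logic lives in Interact.
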(event EventBeginPlay
  (|CallParentFunction) ; This node is disabled and will not be called.\nDrag off pins to build functionality.
)

(event Collision|EventActorBeginOverlap
  (params (OtherActor :type Actor%20Object%20Reference))
  (|CallParentFunction OtherActor) ; This node is disabled and will not be called.\nDrag off pins to build functionality.
)

(event EventTick
  (params (DeltaSeconds :type Float%20%28single-precision%29))
  (|CallParentFunction DeltaSeconds) ; This node is disabled and will not be called.\nDrag off pins to build functionality.
)

(fn ConstructionScript
  (|CallParentFunction))

(fn Interact
  (params (Interactor :type BP%20Lighthouse%20Character%20Object%20Reference))
  (if (not (Variables|/Game/Blueprints/BP_LighthouseCharacter.BP_LighthouseCharacter_C|GetIsCarryingPlank Interactor))
    (Default|SetPlank Interactor true)
    (Actor|DestroyActor)
    (return false)))