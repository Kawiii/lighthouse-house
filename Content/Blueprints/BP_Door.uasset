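; BP_Door is an interactable door that opens only for a character whose inventory contains the required item index.
; Interact flips the interaction state and calls ToggleDoorState, or shows a need-key prompt on the lighthouse character's HUD when the item is missing.
; A timeline drives the door mesh's yaw, playing from start or reversing with the state, and plays a door sound at the mesh when finished.
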(event Custom|ToggleDoorState
  (params (State :type Boolean))
  (if State
    (bind _doorrotation (Timeline|Timeline PlayFromStart)
      (:Update
        (Transformation|SetRelativeRotation (Variables|Default|GetSM_Door) (Math|Rotator|MakeRotator 0.0 0.0 _doorrotation) false false))
      (:Finished
        (Audio|PlaySoundatLocation "/Game/SOUND/Free_Sounds_Pack/Door_Close_4-1.Door_Close_4-1" (Transformation|GetWorldLocation (Variables|Default|GetSM_Door)) "0, 0, 0" 1.0 1.0 0.0 0 0 0 0)))
    (else
      (Timeline|Timeline Reverse))))

(event EventBeginPlay)

(event Collision|EventActorBeginOverlap
  (params (OtherActor :type Actor%20Object%20Reference)))

(event EventTick
  (params (DeltaSeconds :type Float%20%28single-precision%29)))

(fn ConstructionScript
  (|CallParentFunction))

(fn Interact
  (params (Interactor :type BP%20Lighthouse%20Character%20Object%20Reference))
  ;[0.15 0.15 0.15 0.5] Podminka pro vlastnictvi itemu urciteho Indexu
  (bind _output_get (LocalVariables|SetCharacter Interactor))
  (if (Utilities|Array|ContainsItem (Variables|/Game/Blueprints/BP_LighthouseCharacter.BP_LighthouseCharacter_C|GetInventory _output_get) (Variables|Default|GetRequiredItemIndex))
    (bind _output_get_2 (Variables|Default|SetInteractionState (not (Variables|Default|GetInteractionState))))
    (CallFunction|ToggleDoorState self _output_get_2)
    (return (Variables|Default|GetInteractionState))
    (else
      (bind _asbp_lighthouse_character (Utilities|Casting|CastToBP_LighthouseCharacter Interactor))
      (Default|ShowNeedKey (Variables|/Game/Blueprints/BP_LighthouseCharacter.BP_LighthouseCharacter_C|GetHUD_Widget _asbp_lighthouse_character))
      (return false))))

(fn ToggleDoor
  (params (State :type Boolean)))