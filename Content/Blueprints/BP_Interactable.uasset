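; BP_Interactable is a hover-to-collect object that shrinks away and spawns a BP_ItemCompass.
; A Box overlap tracks proximity, which gates cursor hover on the Sphere.
; Hovering plays a timeline that scales the Cube toward zero, and leaving stops it without restoring scale.
; On completion it activates an explosion, waits briefly, spawns the compass at a hard-coded world transform and destroys itself.
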(event OnComponentBeginOverlap(Box)
  (params (OverlappedComponent :type Primitive%20Component%20Object%20Reference) (OtherActor :type Actor%20Object%20Reference) (OtherComp :type Primitive%20Component%20Object%20Reference) (OtherBodyIndex :type Integer) (bFromSweep :type Boolean) (SweepResult :type Hit%20Result%20Structure%20%28by%20ref%29))
  (bind _output_get (Variables|Default|SetbIsPlayerNearby true))
  (Development|PrintString "Hello"))

(event OnComponentEndOverlap(Box)
  (params (OverlappedComponent :type Primitive%20Component%20Object%20Reference) (OtherActor :type Actor%20Object%20Reference) (OtherComp :type Primitive%20Component%20Object%20Reference) (OtherBodyIndex :type Integer))
  (bind _output_get (Variables|Default|SetbIsPlayerNearby false))
  (Development|PrintString "bye"))

(event OnBeginCursorOver(Sphere)
  (params (TouchedComponent :type Primitive%20Component%20Object%20Reference))
  (if (stale OnComponentBeginOverlap(Box) _output_get)
    (Variables|Default|SetOriginalScale (Transformation|GetWorldScale (Variables|Default|GetCube)))
    (bind _scalealpha (Timeline|ShrinkTimeline Play)
      (:Update
        (Development|PrintString "On Begin Cursor Over")
        (Transformation|SetWorldScale3D (Variables|Default|GetCube) (Math|Vector|Lerp(Vector) (Variables|Default|GetOriginalScale) "0, 0, 0" _scalealpha)))
      (:Finished
        (Components|Activation|Activate (Variables|Default|GetExplosion) true)
        (Utilities|FlowControl|Delay 0.5)
        (Game|SpawnActorfromClass "/Game/Blueprints/ItemsInspect/BP_ItemCompass.BP_ItemCompass_C" (Math|Transform|MakeTransform "-2000.000000,2980.000000,295.000000" "-8.672601,164.956535,0.573181" "1.500000,1.500000,1.500000") "Undefined" "MultiplyWithRoot" 0 0)
        (Actor|DestroyActor self)))))

(event OnEndCursorOver(Sphere)
  (params (TouchedComponent :type Primitive%20Component%20Object%20Reference))
  (if (stale OnComponentEndOverlap(Box) _output_get)
    (bind _scalealpha (Timeline|ShrinkTimeline Stop)
      (:Update
        (Development|PrintString "On Begin Cursor Over")
        (Transformation|SetWorldScale3D (Variables|Default|GetCube) (Math|Vector|Lerp(Vector) (Variables|Default|GetOriginalScale) "0, 0, 0" _scalealpha)))
      (:Finished
        (Components|Activation|Activate (Variables|Default|GetExplosion) true)
        (Utilities|FlowControl|Delay 0.5)
        (Game|SpawnActorfromClass "/Game/Blueprints/ItemsInspect/BP_ItemCompass.BP_ItemCompass_C" (Math|Transform|MakeTransform "-2000.000000,2980.000000,295.000000" "-8.672601,164.956535,0.573181" "1.500000,1.500000,1.500000") "Undefined" "MultiplyWithRoot" 0 0)
        (Actor|DestroyActor self)))))

(fn ConstructionScript)