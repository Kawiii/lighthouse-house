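; BP_InteractableBase is a base interactable that offers a text prompt when the lighthouse character enters its range.
; A sphere, sized from Radius at construction, caches the overlapping character and registers itself and InteractionText through SetInteraction.
; End overlap clears the interaction on that cached character without checking which actor left.
; Interact is a placeholder that prints a message and returns false.
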(event OnComponentBeginOverlap(Sphere)
  (params (OverlappedComponent :type Primitive%20Component%20Object%20Reference) (OtherActor :type Actor%20Object%20Reference) (OtherComp :type Primitive%20Component%20Object%20Reference) (OtherBodyIndex :type Integer) (bFromSweep :type Boolean) (SweepResult :type Hit%20Result%20Structure%20%28by%20ref%29))
  (bind _asbp_lighthouse_character (Utilities|Casting|CastToBP_LighthouseCharacter OtherActor))
  (bind _output_get (Variables|Interaction|SetInteractionCharacter _asbp_lighthouse_character))
  (Default|SetInteraction _output_get (Variables|Interaction|GetInteractionText) true self))

(event OnComponentEndOverlap(Sphere)
  (params (OverlappedComponent :type Primitive%20Component%20Object%20Reference) (OtherActor :type Actor%20Object%20Reference) (OtherComp :type Primitive%20Component%20Object%20Reference) (OtherBodyIndex :type Integer))
  (bind _interactioncharacter (Variables|Interaction|GetInteractionCharacter))
  (if (Utilities|IsValid _interactioncharacter)
    (Default|SetInteraction _interactioncharacter "" false self)))

(fn ConstructionScript
  (Components|Sphere|SetSphereRadius (Variables|Default|GetSphere) (Variables|Interaction|GetRadius) true)
  (Variables|Interaction|SetInteractionState false))

(fn Interact
  (params (Interactor :type BP%20Lighthouse%20Character%20Object%20Reference))
  (Development|PrintString "Interaction Functionality Comes Here")
  (return false))