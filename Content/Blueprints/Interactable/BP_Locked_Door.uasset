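; Interactable locked door that swings open and closed for a character carrying the key item.
; Interact checks the interactor's inventory for a hardcoded item index, flips the interaction state and calls ToggleDoorState, or prints a missing-key message.
; ToggleDoorState plays a timeline from the start to open and reverses it to close, driving the door mesh's relative yaw.
; The separate ToggleDoor function is an empty stub.
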(event Custom|ToggleDoorState
  (params (State :type Boolean))
  (if State
    (bind _doorrotation (Timeline|Timeline PlayFromStart)
      (:Update
        (Transformation|SetRelativeRotation (Variables|Default|GetSM_Door) (Math|Rotator|MakeRotator 0.0 0.0 _doorrotation) false false)))
    (else
      (Timeline|Timeline Reverse))))

(event EventBeginPlay)

(event Collision|EventActorBeginOverlap
  (params (OtherActor :type Actor%20Object%20Reference)))

(event EventTick
  (params (DeltaSeconds :type Float%20%28single-precision%29)))

(fn ConstructionScript
  (|CallParentFunction))

(fn Interact
  (params (Interactor :type BP%20Lighthouse%20Character%20Object%20Reference))
  ;[0.15 0.15 0.15 0.5] Podminka pro vlastnictvi itemu urciteho Indexu
  (bind _output_get (LocalVariables|SetCharacter Interactor))
  (if (Utilities|Array|ContainsItem (Variables|/Game/Blueprints/BP_LighthouseCharacter.BP_LighthouseCharacter_C|GetInventory _output_get) 2)
    (bind _output_get_2 (Variables|Default|SetInteractionState (not (Variables|Default|GetInteractionState))))
    (CallFunction|ToggleDoorState self _output_get_2)
    (return (Variables|Default|GetInteractionState))
    (else
      (Development|PrintString "You don't have a key!")
      (return false))))

(fn ToggleDoor
  (params (State :type Boolean)))