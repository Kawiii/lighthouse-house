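; Footprint component that line-traces from a foot socket to the ground and spawns surface-based step sounds and footprint decals, replicated through server and multicast events.
; Physical surfaces set a foot state (muddy, sandy, wet, bloody) that carries onto later surfaces for a limited step count.
; Data tables supply decal materials, matched by footwear and foot for carried prints.
; A dynamic material instance flattens and fades each print as steps accumulate.
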(event Custom|ServerSpawnFootprint
  (params (Location :type Vector) (Rotation :type Rotator) (Decal%20Material :type Material%20Instance%20Object%20Reference) (Current%20Steps :type Float%20%28double-precision%29) (MaxSteps :type Float%20%28double-precision%29))
  ;[1 1 1] Server Spawn Footprint
  (Variables|Default|SetDecal Decal%20Material)
  (bind _returnvalue (Game|SpawnActorfromClass "/Game/Footprints/blueprints/Footprint_Actor.Footprint_Actor_C" (Math|Transform|MakeTransform Location Rotation) "AlwaysSpawn" "OverrideRootScale" 0 0))
  (Variables|Default|SetFootprintActor _returnvalue)
  (Utilities|FlowControl|Delay 0.1)
  (CallFunction|MulticastFootprintMaterial (Variables|Default|GetDecal) (Variables|Default|GetFootprintActor) Current%20Steps MaxSteps))

(event Custom|MulticastFootprintMaterial
  (params (Decal%20Material :type Material%20Instance%20Object%20Reference) (Footprint%20Actor :type Footprint%20Actor%20Object%20Reference) (CurrentSteps :type Float%20%28double-precision%29) (MaxSteps :type Float%20%28double-precision%29))
  ;[1 1 1] Multicast Footprint Info
  (Variables|Default|SetDecal Decal%20Material)
  (bind _output_get (Variables|Default|SetFootprintActor Footprint%20Actor))
  (Utilities|IsValid _output_get
    (:Is%20Valid
      (Variables|Default|SetCurrentMulticastSteps CurrentSteps)
      (Variables|Default|SetCurrentMaxSteps MaxSteps)
      (Rendering|Components|Decal|SetDecalMaterial (Variables|/Game/Footprints/blueprints/Footprint_Actor.Footprint_Actor_C|GetFootprintDecal (Variables|Default|GetFootprintActor)) (Variables|Default|GetDecal))
      (bind _returnvalue (Rendering|Material|CreateDynamicMaterialInstance (Variables|/Game/Footprints/blueprints/Footprint_Actor.Footprint_Actor_C|GetFootprintDecal (Variables|Default|GetFootprintActor)) :!class /Script/Engine.DecalComponent))
      (Rendering|Material|SetScalarParameterValue _returnvalue "Flatness" (/ (Variables|Default|GetCurrentMulticastSteps) (Variables|Default|GetCurrentMaxSteps)) :!class /Script/Engine.MaterialInstanceDynamic)
      (Rendering|Material|SetScalarParameterValue _returnvalue "Opacityness" (- 1.0 (/ (Variables|Default|GetCurrentMulticastSteps) (Variables|Default|GetCurrentMaxSteps))) :!class /Script/Engine.MaterialInstanceDynamic)
      (Rendering|SetVisibility (Variables|/Game/Footprints/blueprints/Footprint_Actor.Footprint_Actor_C|GetFootprintDecal (Variables|Default|GetFootprintActor)) true false))))

(event Custom|MulticastSpawnSound
  (params (Sound :type Sound%20Base%20Object%20Reference) (Location :type Vector))
  ;[1 1 1] Multicast Sound
  (Audio|PlaySoundatLocation Sound Location "0, 0, 0" 1.0 (Math|Random|RandomFloatinRange 0.8 1.2) 0.0 "/Game/Footprints/Sounds/StepAttenuation.StepAttenuation" 0 0 0))

(event Custom|ServerSpawnSound
  (params (Sound :type Sound%20Base%20Object%20Reference) (Location :type Vector))
  ;[1 1 1] Server Spawn Sound
  (CallFunction|MulticastSpawnSound Sound Location))

(event EventSpawnDecal
  (params (SocketName :type Name :default "None") (Right :type Boolean) (Left :type Boolean))
  (bind _mesh (Variables|Default|GetMesh))
  (bind _returnvalue (Transformation|GetSocketLocation _mesh SocketName))
  ;[1 1 1] Line Trace to Ground
  (bind (_outhit _returnvalue_2) (Collision|LineTraceByChannel (+ _returnvalue "0, 0,150.000000") (- _returnvalue "0, 0,50.000000") "TraceTypeQuery1" false 0 "None"))
  (if _returnvalue_2
    (Utilities|IsValid (.PhysMat (Collision|BreakHitResult _outhit))
      (:Is%20Valid
        (CallFunction|SpawnFootprint (.Location (Collision|BreakHitResult _outhit)) (Math|Rotator|MakeRotator 0.0 (.Pitch (Math|Rotator|BreakRotator (Math|Conversions|RotationFromXVector (Math|Vector|NegateVector (.ImpactNormal (Collision|BreakHitResult _outhit)))))) (.Yaw (Math|Rotator|BreakRotator (Math|Conversions|RotationFromXVector (Math|Vector|GetForwardVector (Variables|Default|GetMesh)))))) Right Left (Variables|/Script/PhysicsCore.PhysicalMaterial|GetSurfaceType (.PhysMat (Collision|BreakHitResult _outhit))))))))

(fn SpawnFootprint
  (params (Location :type Vector) (Rotation :type Rotator) (Left :type Boolean) (Right :type Boolean) (SurfaceType :type EPhysicalSurface%20Enum :default "SurfaceType_Default"))
  (bind _currentfootwear (Variables|Default|GetCurrentFootwear))
  (bind _currentfootwear_2 (Variables|Default|GetCurrentFootwear))
  (bind _currentfootwear_3 (Variables|Default|GetCurrentFootwear))
  (bind _currentfootwear_4 (Variables|Default|GetCurrentFootwear))
  (bind _currentfootwear_5 (Variables|Default|GetCurrentFootwear))
  ;[1 1 1] Setting various Variables
  (Variables|Default|SetLocation Location)
  (Variables|Default|SetRotation Rotation)
  (Variables|Default|SetLeft Left)
  (Variables|Default|SetRight Right)
  ;[1 1 1] Determins on which SurfaceType a Decal should Spawn
  (switch Utilities|FlowControl|Switch|SwitchonEPhysicalSurface SurfaceType
    (:SurfaceType_Default
      ;[1 1 1] Basic Sounds - You can use a CurrentFootwear test here to use sounds according to your Footwear and the Ground
      (CallFunction|ServerSpawnSound "/Game/Footprints/Sounds/Stone.Stone" (Variables|Default|GetLocation) :!label _label)
      ;[1 1 1] Check current FootState
      (switch Utilities|FlowControl|Switch|SwitchonEFootState (Variables|Default|GetFootState) :!label _label_2
        (:NewEnumerator1
          ;[1 1 1] Adjusting FootState or Check Database for the correct Material in this situation
          (if (>= (Variables|Default|GetCurrentMudSteps) (Variables|Default|GetMaxMudSteps))
            (Variables|Default|SetFootState "NewEnumerator0")
            (Variables|Default|SetCurrentMudSteps 0.0)
            (else
              (Math|Float|IncrementFloat (Variables|Default|GetCurrentMudSteps)
                (:%20%20
                  (bind _outrownames (DataTable|GetDataTableRowNames "/Game/Footprints/blueprints/Data/FootprintMudyDataTable.FootprintMudyDataTable"))
                  (for _array_element _outrownames
                    (bind _returnvalue (Utilities|GetDataTableRow "/Game/Footprints/blueprints/Data/FootprintMudyDataTable.FootprintMudyDataTable" _array_element)
                      (:then
                        (if (or (and (== (.Style (Utilities|Struct|BreakFootprintModifyStruct _returnvalue)) _currentfootwear) (Math|Boolean|Equal(Boolean) (.Right (Utilities|Struct|BreakFootprintModifyStruct _returnvalue)) (Variables|Default|GetRight))) (and (== (.Style (Utilities|Struct|BreakFootprintModifyStruct _returnvalue)) _currentfootwear) (Math|Boolean|Equal(Boolean) (.Left (Utilities|Struct|BreakFootprintModifyStruct _returnvalue)) (Variables|Default|GetLeft))))
                          (CallFunction|ServerSpawnFootprint (Variables|Default|GetLocation) (Variables|Default|GetRotation) (.MaterialInterface (Utilities|Struct|BreakFootprintModifyStruct _returnvalue)) (Variables|Default|GetCurrentMudSteps) (Variables|Default|GetMaxMudSteps)))))))))))
        (:NewEnumerator2
          ;[1 1 1] Adjusting FootState or Check Database for the correct Material in this situation
          (if (>= (Variables|Default|GetCurrentSandSteps) (Variables|Default|GetMaxSandSteps))
            (Variables|Default|SetFootState "NewEnumerator0")
            (Variables|Default|SetCurrentSandSteps 0.0)
            (else
              (Math|Float|IncrementFloat (Variables|Default|GetCurrentSandSteps)
                (:%20%20
                  (bind _outrownames_2 (DataTable|GetDataTableRowNames "/Game/Footprints/blueprints/Data/FootprintSandyDataTable.FootprintSandyDataTable"))
                  (for _array_element_2 _outrownames_2
                    (bind _returnvalue_2 (Utilities|GetDataTableRow "/Game/Footprints/blueprints/Data/FootprintSandyDataTable.FootprintSandyDataTable" _array_element_2)
                      (:then
                        (if (or (and (== (.Style (Utilities|Struct|BreakFootprintModifyStruct _returnvalue_2)) _currentfootwear_2) (Math|Boolean|Equal(Boolean) (.Right (Utilities|Struct|BreakFootprintModifyStruct _returnvalue_2)) (Variables|Default|GetRight))) (and (== (.Style (Utilities|Struct|BreakFootprintModifyStruct _returnvalue_2)) _currentfootwear_2) (Math|Boolean|Equal(Boolean) (.Left (Utilities|Struct|BreakFootprintModifyStruct _returnvalue_2)) (Variables|Default|GetLeft))))
                          (CallFunction|ServerSpawnFootprint (Variables|Default|GetLocation) (Variables|Default|GetRotation) (.MaterialInterface (Utilities|Struct|BreakFootprintModifyStruct _returnvalue_2)) (Variables|Default|GetCurrentSandSteps) (Variables|Default|GetMaxSandSteps)))))))))))
        (:NewEnumerator3
          ;[1 1 1] Adjusting FootState or Check Database for the correct Material in this situation
          (if (>= (Variables|Default|GetCurrentWetSteps) (Variables|Default|GetMaxWetSteps))
            (Variables|Default|SetFootState "NewEnumerator0")
            (Variables|Default|SetCurrentWetSteps 0.0)
            (else
              (Math|Float|IncrementFloat (Variables|Default|GetCurrentWetSteps)
                (:%20%20
                  (bind _outrownames_3 (DataTable|GetDataTableRowNames "/Game/Footprints/blueprints/Data/FootprintWetDataTable.FootprintWetDataTable"))
                  (for _array_element_3 _outrownames_3
                    (bind _returnvalue_3 (Utilities|GetDataTableRow "/Game/Footprints/blueprints/Data/FootprintWetDataTable.FootprintWetDataTable" _array_element_3)
                      (:then
                        (if (or (and (== (.Style (Utilities|Struct|BreakFootprintModifyStruct _returnvalue_3)) _currentfootwear_3) (Math|Boolean|Equal(Boolean) (.Right (Utilities|Struct|BreakFootprintModifyStruct _returnvalue_3)) (Variables|Default|GetRight))) (and (== (.Style (Utilities|Struct|BreakFootprintModifyStruct _returnvalue_3)) _currentfootwear_3) (Math|Boolean|Equal(Boolean) (.Left (Utilities|Struct|BreakFootprintModifyStruct _returnvalue_3)) (Variables|Default|GetLeft))))
                          (CallFunction|ServerSpawnFootprint (Variables|Default|GetLocation) (Variables|Default|GetRotation) (.MaterialInterface (Utilities|Struct|BreakFootprintModifyStruct _returnvalue_3)) (Variables|Default|GetCurrentWetSteps) (Variables|Default|GetMaxWetSteps)))))))))))
        (:NewEnumerator4
          ;[1 1 1] Adjusting FootState or Check Database for the correct Material in this situation
          (if (>= (Variables|Default|GetCurrentBloodSteps) (Variables|Default|GetMaxBloodSteps))
            (Variables|Default|SetFootState "NewEnumerator0")
            (Variables|Default|SetCurrentBloodSteps 0.0)
            (else
              (Math|Float|IncrementFloat (Variables|Default|GetCurrentBloodSteps)
                (:%20%20
                  (bind _outrownames_4 (DataTable|GetDataTableRowNames "/Game/Footprints/blueprints/Data/FootprintBloodyDataTable.FootprintBloodyDataTable"))
                  (for _array_element_4 _outrownames_4
                    (bind _returnvalue_4 (Utilities|GetDataTableRow "/Game/Footprints/blueprints/Data/FootprintBloodyDataTable.FootprintBloodyDataTable" _array_element_4)
                      (:then
                        (if (or (and (== (.Style (Utilities|Struct|BreakFootprintModifyStruct _returnvalue_4)) _currentfootwear_5) (Math|Boolean|Equal(Boolean) (.Right (Utilities|Struct|BreakFootprintModifyStruct _returnvalue_4)) (Variables|Default|GetRight))) (and (== (.Style (Utilities|Struct|BreakFootprintModifyStruct _returnvalue_4)) _currentfootwear_5) (Math|Boolean|Equal(Boolean) (.Left (Utilities|Struct|BreakFootprintModifyStruct _returnvalue_4)) (Variables|Default|GetLeft))))
                          (CallFunction|ServerSpawnFootprint (Variables|Default|GetLocation) (Variables|Default|GetRotation) (.MaterialInterface (Utilities|Struct|BreakFootprintModifyStruct _returnvalue_4)) (Variables|Default|GetCurrentBloodSteps) (Variables|Default|GetMaxBloodSteps)))))))))))))
    (:SurfaceType1
      (CallFunction|ServerSpawnSound "/Game/Footprints/Sounds/Sand.Sand" (Variables|Default|GetLocation))
      ;[1 1 1] Setting State Parameters and Current Step
      (Variables|Default|SetFootState "NewEnumerator2")
      (Variables|Default|SetCurrentSandSteps 0.0)
      ;[1 1 1] Check Database for the correct Material in this situation
      (bind _outrownames_5 (DataTable|GetDataTableRowNames "/Game/Footprints/blueprints/Data/FootprintDataTable.FootprintDataTable" :!label _label_3))
      (for _array_element_5 _outrownames_5
        (bind _returnvalue_5 (Utilities|GetDataTableRow "/Game/Footprints/blueprints/Data/FootprintDataTable.FootprintDataTable" _array_element_5)
          (:then
            (if (or (and (== (.Style (Utilities|Struct|BreakFootprintModifyStruct _returnvalue_5)) _currentfootwear_4) (Math|Boolean|Equal(Boolean) (.Right (Utilities|Struct|BreakFootprintModifyStruct _returnvalue_5)) (Variables|Default|GetRight))) (and (== (.Style (Utilities|Struct|BreakFootprintModifyStruct _returnvalue_5)) _currentfootwear_4) (Math|Boolean|Equal(Boolean) (.Left (Utilities|Struct|BreakFootprintModifyStruct _returnvalue_5)) (Variables|Default|GetLeft))))
              _
              (else
                _))
            ;[1 1 1] Spawn Footprint Actor with correct Material
            (CallFunction|ServerSpawnFootprint (Variables|Default|GetLocation) (Variables|Default|GetRotation) (.MaterialInterface (Utilities|Struct|BreakFootprintModifyStruct _returnvalue_5)) 0.0 1e+02)))))
    (:SurfaceType2
      (goto _label))
    (:SurfaceType3
      (CallFunction|ServerSpawnSound "/Game/Footprints/Sounds/S_Snow.S_Snow" (Variables|Default|GetLocation))
      (Variables|Default|SetFootState "NewEnumerator1")
      (Variables|Default|SetCurrentMudSteps 0.0)
      (goto _label_3))
    (:SurfaceType4
      (CallFunction|ServerSpawnSound "/Game/Footprints/Sounds/Water.Water" (Variables|Default|GetLocation))
      ;[1 1 1] Not Spawning Any Footprints for Water
      (Variables|Default|SetFootState "NewEnumerator3")
      (Variables|Default|SetCurrentWetSteps 0.0))
    (:SurfaceType5
      (CallFunction|ServerSpawnSound "/Game/Footprints/Sounds/Blood.Blood" (Variables|Default|GetLocation))
      ;[1 1 1] Special Blood Treatment
      (Variables|Default|SetFootState "NewEnumerator4")
      (Variables|Default|SetCurrentBloodSteps 0.0)
      (goto _label_2))))