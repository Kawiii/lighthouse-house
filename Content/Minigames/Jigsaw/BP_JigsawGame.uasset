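; Interactable jigsaw minigame actor that starts the puzzle and leaves a photo item in the level.
; The construction script sizes its sphere from a radius variable and clears the interaction state.
; Interact calls PlayJigsaw on the interactor, destroys the actor and immediately spawns BP_ItemPhoto, without waiting for a puzzle result.
; The photo appears at the first TargetPoint returned by a level-wide class search, so placement depends on that lookup.
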(fn ConstructionScript
  (Components|Sphere|SetSphereRadius (Variables|Default|GetSphere) (Variables|Default|GetRadius_0) true)
  (Variables|Default|SetInteractionState_0 false))

(fn Interact
  (params (Interactor :type BP%20Lighthouse%20Character%20Object%20Reference))
  (Default|PlayJigsaw Interactor)
  (Actor|DestroyActor)
  (bind _outactors (Actor|GetAllActorsOfClass "/Script/Engine.TargetPoint"))
  (Game|SpawnActorfromClass "/Game/Blueprints/ItemsInspect/BP_ItemPhoto.BP_ItemPhoto_C" (Math|Transform|MakeTransform (Transformation|GetActorLocation (Utilities|Array|Get(acopy) _outactors))) "Undefined" "MultiplyWithRoot" 0 false 0 0 0)
  (return true))